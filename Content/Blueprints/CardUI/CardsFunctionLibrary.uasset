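; Blueprint function library for the card game, giving shared access to the player's cards and a helper for card UI movement.
; Deck and discard getters cast the game mode to CardGameMode and return its piles, and a random-card getter draws on the deck without removing the card.
; The interpolation helper eases a widget transform's translation and angle toward a destination, leaving scale and shear at MakeWidgetTransform defaults.
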(fn GetRandomCard
  (return (.OutItem (Utilities|Array|Random (CallFunction|GetPlayerDeck)))))

(fn InterpolateTowardsPosition
  (params (Current%20Position :type Widget%20Transform%20Structure) (Destination%20Transform :type Widget%20Transform%20Structure) (Delta :type Float%20%28double-precision%29) (Interpolation%20Speed :type Float%20%28double-precision%29))
  (bind (_translation _scale _shear _angle) (Utilities|Struct|BreakWidgetTransform Current%20Position))
  (bind (_translation_2 _scale_2 _shear_2 _angle_2) (Utilities|Struct|BreakWidgetTransform Destination%20Transform))
  (return (Utilities|Struct|MakeWidgetTransform (Class|KismetMathLibrary|Vector2DInterpto _translation _translation_2 Delta Interpolation%20Speed) "(X=1.000000,Y=1.000000)" "(X=0.000000,Y=0.000000)" (Math|Interpolation|FInterpTo _angle _angle_2 Delta Interpolation%20Speed))))

(fn GetPlayerDeck
  (bind _ascard_game_mode (Utilities|Casting|CastToCardGameMode (Game|GetGameMode)))
  (return (Variables|/Game/Blueprints/CardUI/CardGameMode.CardGameMode_C|GetPlayerDeck _ascard_game_mode)))

(fn GetPlayerDiscard
  (bind _ascard_game_mode (Utilities|Casting|CastToCardGameMode (Game|GetGameMode)))
  (return (Variables|/Game/Blueprints/CardUI/CardGameMode.CardGameMode_C|GetPlayerDiscard _ascard_game_mode)))