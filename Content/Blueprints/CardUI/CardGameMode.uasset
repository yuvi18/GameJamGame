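; CardGameMode is a game mode Blueprint that tracks whose turn it is in a card game, player or enemy.
; End Turn passes the turn from player to enemy, and Start Turn passes it back, each only from the matching state.
; A separate TurnSwitch event prints the current turn to screen as debug text; neither function calls it.
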(event Custom|TurnSwitch
  (switch Utilities|FlowControl|Switch|SwitchonTurnEnums (Variables|Default|GetCurrentTurn)
    (:NewEnumerator0
      (Development|PrintString "Player Turn"))
    (:NewEnumerator1
      (Development|PrintString "Enemy Turn"))))

(event EventBeginPlay)

(event EventTick
  (params (DeltaSeconds :type Float%20%28single-precision%29)))

(fn ConstructionScript)

(fn EndTurn
  (if (Utilities|Enum|Equal(Enum) (Variables|Default|GetCurrentTurn) "NewEnumerator0")
    (Variables|Default|SetCurrentTurn "NewEnumerator1")))

(fn StartTurn
  (if (Utilities|Enum|Equal(Enum) (Variables|Default|GetCurrentTurn) "NewEnumerator1")
    (Variables|Default|SetCurrentTurn "NewEnumerator0")))